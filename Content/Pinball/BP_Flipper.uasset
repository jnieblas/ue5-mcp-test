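; Pinball flipper actor that swings PivotArm between rest and flip yaw from polled keyboard input, with IsRight selecting right or left keys.
; Tick holds the flip while a key is down or a short press timer runs, easing the angle at constant speed.
; Hits on "Ball"-tagged actors during flips add velocity only when IsRight, via two chained impulses whose sideways components cancel.
; Older hit and tick variants remain unconnected.
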(event `self.ReceiveBeginPlay`
  (`self.EnableInput` self (`GameplayStatics.GetPlayerController` 0))
  (set `self.CurrentAngle` (`self.RestAngle`))
  (`SceneComponent.K2_SetRelativeRotation` (`self.PivotArm`) (`KismetMathLibrary.MakeRotator` 0.0 0.0 (`self.RestAngle`)) false false))

(event `self.ReceiveTick`
  (params (DeltaSeconds :type "Float (single-precision)"))
  (bind _returnvalue (`GameplayStatics.GetPlayerController` 0))
  (bind _returnvalue_2 (or (select `bool` (`self.IsRight`) :`false` (or (`PlayerController.IsInputKeyDown` _returnvalue "Left") (`PlayerController.IsInputKeyDown` _returnvalue "A")) :`true` (or (`PlayerController.IsInputKeyDown` _returnvalue "Right") (`PlayerController.IsInputKeyDown` _returnvalue "D"))) (> (`self.FlipTimer`) 0.0)))
  (bind _returnvalue_3 (`KismetMathLibrary.FInterpTo_Constant` (`self.CurrentAngle`) (select `bool` _returnvalue_2 :`false` (`self.RestAngle`) :`true` (`self.FlipAngle`)) DeltaSeconds 700.0))
  (if (select `bool` (`self.IsRight`) :`false` (or (`PlayerController.WasInputKeyJustPressed` _returnvalue "Left") (`PlayerController.WasInputKeyJustPressed` _returnvalue "A")) :`true` (or (`PlayerController.WasInputKeyJustPressed` _returnvalue "Right") (`PlayerController.WasInputKeyJustPressed` _returnvalue "D")))
    (set `self.FlipTimer` 0.4))
  (set `self.FlipTimer` (select `bool` (> (- (`self.FlipTimer`) DeltaSeconds) 0.0) :`false` 0.0 :`true` (- (`self.FlipTimer`) DeltaSeconds)))
  (set `self.IsFlipping` _returnvalue_2)
  (set `self.CurrentAngle` _returnvalue_3)
  (`SceneComponent.K2_SetRelativeRotation` (`self.PivotArm`) (`KismetMathLibrary.MakeRotator` 0.0 0.0 _returnvalue_3) false false))

(event `self.ReceiveHit`
  (params (MyComp :type "PrimitiveComponent Object Reference") (Other :type "Actor Object Reference") (OtherComp :type "PrimitiveComponent Object Reference") (bSelfMoved :type Boolean) (HitLocation :type "Vector Structure") (HitNormal :type "Vector Structure") (NormalImpulse :type "Vector Structure") (Hit :type "HitResult Structure (by ref)"))
  (if (and (`self.IsFlipping`) (`self.ActorHasTag` Other "Ball"))
    (if (`self.IsRight`)
      (`PrimitiveComponent.AddImpulse` OtherComp (`KismetMathLibrary.MakeVector` 1400.0 -300.0) "None" true)
      (`PrimitiveComponent.AddImpulse` OtherComp (`KismetMathLibrary.MakeVector` 1400.0 300.0) "None" true))))

(fn `UserConstructionScript`
  (`SceneComponent.K2_SetRelativeRotation` (`self.PivotArm`) (`KismetMathLibrary.MakeRotator` 0.0 0.0 (`self.RestAngle`)) false false))