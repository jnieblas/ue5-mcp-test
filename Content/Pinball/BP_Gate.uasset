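; Pinball gate actor that opens and closes according to where the BP_Ball is on the table.
; Each Tick it looks up the ball and compares its X/Y position to hard-coded world thresholds, using no collision or overlap events.
; A GateClosed flag limits moves to state changes, which snap the gate between fixed world positions: sunk below to open, raised to close.
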(event `self.ReceiveBeginPlay`
  (set `self.GateClosed` true))

(event `self.ReceiveTick`
  (params (DeltaSeconds :type "Float (single-precision)"))
  (bind _returnvalue (`GameplayStatics.GetActorOfClass` "/Game/Pinball/BP_Ball.BP_Ball_C"))
  (bind _returnvalue_2 (`self.K2_GetActorLocation` _returnvalue))
  (if (and (`self.GateClosed`) (and (< (.x _returnvalue_2) 10050.0) (> (.y _returnvalue_2) 510.0)))
    (set `self.GateClosed` false)
    (`self.K2_SetActorLocation` (`KismetMathLibrary.MakeVector` 10154.0 590.0 -500.0)))
  (if (and (not (`self.GateClosed`)) (or (< (.y _returnvalue_2) 480.0) (> (.x _returnvalue_2) 10280.0)))
    (set `self.GateClosed` true)
    (`self.K2_SetActorLocation` (`KismetMathLibrary.MakeVector` 10154.0 590.0 50.0))))

(fn `UserConstructionScript`)