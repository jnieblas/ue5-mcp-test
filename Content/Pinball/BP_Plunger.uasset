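; BP_Plunger is the pinball plunger actor, animating its Rod as the player charges a pull.
; Tick polls Space on player controller 0, ramping VisCharge to full while held and easing it back at constant speed on release.
; VisCharge drives the Rod's relative X offset to draw it back.
; The charge is visual only here; this Blueprint applies no force to a ball.
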(event `self.ReceiveBeginPlay`
  (`self.EnableInput` self (`GameplayStatics.GetPlayerController` 0)))

(event `self.ReceiveTick`
  (params (DeltaSeconds :type "Float (single-precision)"))
  (bind _vischarge (`self.VisCharge`))
  (bind _returnvalue (+ _vischarge (/ DeltaSeconds 1.2)))
  (if (`PlayerController.IsInputKeyDown` (`GameplayStatics.GetPlayerController` 0) "SpaceBar")
    (set `self.VisCharge` (select `bool` (> _returnvalue 1.0) :`false` _returnvalue :`true` 1.0))
    (else
      (set `self.VisCharge` (`KismetMathLibrary.FInterpTo_Constant` _vischarge 0.0 DeltaSeconds 6.0))))
  (`SceneComponent.K2_SetRelativeLocation` (`self.Rod`) (`KismetMathLibrary.MakeVector` (- -45.0 (* 70.0 (`self.VisCharge`))) 0.0 10.0) false false))

(fn `UserConstructionScript`)