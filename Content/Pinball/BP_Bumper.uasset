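; Pinball bumper actor that kicks the ball away when the ball strikes it hard enough.
; On Hit, an actor tagged Ball with a strong enough normal impulse receives a fixed-speed velocity-change impulse directed outward from the bumper's location.
; A short PopTimer cooldown, set on each pop and counted down to zero on Tick, blocks repeat kicks.
; Several unconnected leftover variants of the kick logic never run.
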(event `self.ReceiveHit`
  (params (MyComp :type "PrimitiveComponent Object Reference") (Other :type "Actor Object Reference") (OtherComp :type "PrimitiveComponent Object Reference") (bSelfMoved :type Boolean) (HitLocation :type "Vector Structure") (HitNormal :type "Vector Structure") (NormalImpulse :type "Vector Structure") (Hit :type "HitResult Structure (by ref)"))
  (if (and (and (`self.ActorHasTag` Other "Ball") (< (`self.PopTimer`) 0.001)) (> (`KismetMathLibrary.VSize` NormalImpulse) 10000.0))
    (set `self.PopTimer` 0.3)
    (`PrimitiveComponent.AddImpulse` OtherComp (* (`KismetMathLibrary.GetDirectionUnitVector` (`self.K2_GetActorLocation`) (`self.K2_GetActorLocation` Other)) (`KismetMathLibrary.MakeVector` 700.0 700.0 700.0)) "None" true)))

(event `self.ReceiveTick`
  (params (DeltaSeconds :type "Float (single-precision)"))
  (set `self.PopTimer` (select `bool` (> (- (`self.PopTimer`) DeltaSeconds) 0.0) :`false` 0.0 :`true` (- (`self.PopTimer`) DeltaSeconds))))

(fn `UserConstructionScript`)