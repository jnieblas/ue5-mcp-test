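; Pinball ball that handles its own plunger launch, table physics and respawn.
; Holding Space charges a launch impulse along +X, fired on release.
; In play, Tick applies constant -X acceleration as table slope, resets the ball when it drains or settles in the launch lane, and nudges stalled balls toward a fixed point.
; Hit events mirror velocity off the surface normal unless the other actor is tagged "Active".
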(event `self.ReceiveBeginPlay`
  (`self.EnableInput` self (`GameplayStatics.GetPlayerController` 0))
  (`PrimitiveComponent.SetPhysicsLinearVelocity` (`self.Ball`) (`KismetMathLibrary.MakeVector` 0.0) false "None")
  (`self.K2_SetActorLocation` (`KismetMathLibrary.MakeVector` 9320.0 580.0 50.0))
  (set `self.ReadyToLaunch` true))

(event `self.ReceiveTick`
  (params (DeltaSeconds :type "Float (single-precision)"))
  (bind _returnvalue (`self.K2_GetActorLocation`))
  (bind _returnvalue_2 (`GameplayStatics.GetPlayerController` 0))
  (bind _returnvalue_3 (`PlayerController.IsInputKeyDown` _returnvalue_2 "SpaceBar"))
  (bind _returnvalue_4 (`PlayerController.WasInputKeyJustPressed` _returnvalue_2 "SpaceBar"))
  (bind _returnvalue_5 (+ (`self.LaunchCharge`) (/ DeltaSeconds 1.2)))
  (if (`self.ReadyToLaunch`)
    (if _returnvalue_4
      (set `self.IsCharging` true))
    (if (and (`self.IsCharging`) _returnvalue_3)
      (set `self.LaunchCharge` (select `bool` (> _returnvalue_5 1.0) :`false` _returnvalue_5 :`true` 1.0)))
    (if (and (`self.IsCharging`) (or (`PlayerController.WasInputKeyJustReleased` _returnvalue_2 "SpaceBar") (and (not _returnvalue_3) (not _returnvalue_4))))
      (set `self.IsCharging` false)
      (set `self.ReadyToLaunch` false)
      (`PrimitiveComponent.AddImpulse` (`self.Ball`) (`KismetMathLibrary.MakeVector` (`KismetMathLibrary.Lerp` 900.0 2200.0 (`self.LaunchCharge`))) "None" true)
      (set `self.LaunchCharge` 0.0))
    (else
      (`PrimitiveComponent.AddForce` (`self.Ball`) (`KismetMathLibrary.MakeVector` -900.0) "None" true)
      (bind _returnvalue_6 (`PrimitiveComponent.GetPhysicsLinearVelocity` (`self.Ball`) "None"))
      (if (< (.x _returnvalue) 9180.0)
        (`PrimitiveComponent.SetPhysicsLinearVelocity` (`self.Ball`) (`KismetMathLibrary.MakeVector` 0.0) false "None")
        (`self.K2_SetActorLocation` (`KismetMathLibrary.MakeVector` 9320.0 580.0 50.0))
        (set `self.ReadyToLaunch` true)
        (else
          (bind _returnvalue_7 (`KismetMathLibrary.VSize` _returnvalue_6))
          (if (and (and (< (.x _returnvalue) 9345.0) (> (.y _returnvalue) 520.0)) (< _returnvalue_7 80.0))
            (`PrimitiveComponent.SetPhysicsLinearVelocity` (`self.Ball`) (`KismetMathLibrary.MakeVector` 0.0) false "None")
            (`self.K2_SetActorLocation` (`KismetMathLibrary.MakeVector` 9320.0 580.0 50.0))
            (set `self.ReadyToLaunch` true)
            (elif (< _returnvalue_7 60.0)
              (`PrimitiveComponent.SetPhysicsLinearVelocity` (`self.Ball`) (* (`KismetMathLibrary.GetDirectionUnitVector` _returnvalue (`KismetMathLibrary.MakeVector` 9000.0 0.0 50.0)) (`KismetMathLibrary.MakeVector` 500.0 500.0 500.0)) false "None"))))))))

(event `self.ReceiveHit`
  (params (MyComp :type "PrimitiveComponent Object Reference") (Other :type "Actor Object Reference") (OtherComp :type "PrimitiveComponent Object Reference") (bSelfMoved :type Boolean) (HitLocation :type "Vector Structure") (HitNormal :type "Vector Structure") (NormalImpulse :type "Vector Structure") (Hit :type "HitResult Structure (by ref)"))
  (if (not (`self.ActorHasTag` Other "Active"))
    (bind _returnvalue (`PrimitiveComponent.GetPhysicsLinearVelocity` (`self.Ball`) "None"))
    (`PrimitiveComponent.SetPhysicsLinearVelocity` (`self.Ball`) (`KismetMathLibrary.MirrorVectorByNormal` _returnvalue HitNormal) false "None")))

(fn `UserConstructionScript`)